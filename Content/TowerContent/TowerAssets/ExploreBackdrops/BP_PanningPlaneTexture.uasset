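; Backdrop actor that displays a texture on a plane with configurable panning and color tint.
; The construction script feeds the texture, pan speeds and tint into a dynamic material instance on the plane.
; It sizes the plane and box from the texture's pixel dimensions and offsets both by the centering mode, using half-unit nudges for odd sizes when centered.
; BeginPlay reapplies the tint color through UpdateTint.
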(event EventBeginPlay
  (CallFunction|UpdateTint))

(event Collision|EventActorBeginOverlap
  (params (OtherActor :type Actor%20Object%20Reference)))

(event EventTick
  (params (DeltaSeconds :type Float%20%28single-precision%29)))

(fn ConstructionScript
  (bind _texture (Variables|Rendering|GetTexture))
  (bind _texture_2 (Variables|Rendering|GetTexture))
  (bind _returnvalue (Rendering|Material|CreateDynamicMaterialInstance (Variables|Rendering|GetMaterial) "None" "None" :!class /Script/Engine.KismetMaterialLibrary))
  (Variables|Default|SetDynamicMaterialInstance _returnvalue)
  (Rendering|Material|SetTextureParameterValue (Variables|Default|GetDynamicMaterialInstance) "PlaneTexture" (Variables|Rendering|GetTexture))
  (Rendering|Material|SetScalarParameterValue (Variables|Default|GetDynamicMaterialInstance) "PanningYSpeed" (Variables|Rendering|GetPanningY) :!class /Script/Engine.MaterialInstanceDynamic)
  (Rendering|Material|SetScalarParameterValue (Variables|Default|GetDynamicMaterialInstance) "PanningXSpeed" (Variables|Rendering|GetPanningX) :!class /Script/Engine.MaterialInstanceDynamic)
  (Rendering|Material|SetScalarParameterValue (Variables|Default|GetDynamicMaterialInstance) "TintIntensity" (Variables|Rendering|GetTintIntensity) :!class /Script/Engine.MaterialInstanceDynamic)
  (Rendering|Material|SetVectorParameterValue (Variables|Default|GetDynamicMaterialInstance) "TintColor" (Variables|Rendering|GetTintColor) :!class /Script/Engine.MaterialInstanceDynamic)
  (Rendering|Material|SetMaterial (Variables|Default|GetPlane) 0 (Variables|Default|GetDynamicMaterialInstance))
  (LocalVariables|SetNewScale (Math|Vector|MakeVector (/ (Math|Conversions|ToFloat(Integer) (Class|Texture2D|BlueprintGetSizeX _texture_2)) 1e+02) (/ (Math|Conversions|ToFloat(Integer) (Class|Texture2D|BlueprintGetSizeY _texture_2)) 1e+02) 1.0))
  (Transformation|SetRelativeScale3D (Variables|Default|GetPlane) (LocalVariables|GetNewScale))
  (Components|Box|SetBoxExtent (Variables|Default|GetBox) (* (LocalVariables|GetNewScale) 5e+01) false)
  (LocalVariables|SetNewOffset (Utilities|Select :Index (Variables|Rendering|GetCentering) :NewEnumerator2 (Math|Vector|MakeVector 0.0 (/ (Math|Conversions|ToFloat(Integer) (Class|Texture2D|BlueprintGetSizeY (Variables|Rendering|GetTexture))) 2.0) 0.0) :NewEnumerator0 (Math|Vector|MakeVector (select (> (Math|Integer|%(Integer) (Class|Texture2D|BlueprintGetSizeX _texture) 2) 0) 0.5 0.0) (select (> (Math|Integer|%(Integer) (Class|Texture2D|BlueprintGetSizeY _texture) 2) 0) 0.5 0.0) 0.0) :NewEnumerator1 (Math|Vector|MakeVector 0.0 (* (/ (Math|Conversions|ToFloat(Integer) (Class|Texture2D|BlueprintGetSizeY (Variables|Rendering|GetTexture))) 2.0) -1.0) 0.0) :NewEnumerator3 (Math|Vector|MakeVector (/ (Math|Conversions|ToFloat(Integer) (Class|Texture2D|BlueprintGetSizeX (Variables|Rendering|GetTexture))) 2.0) (* (/ (Math|Conversions|ToFloat(Integer) (Class|Texture2D|BlueprintGetSizeY (Variables|Rendering|GetTexture))) 2.0) -1.0) 0.0)))
  (Transformation|SetRelativeLocation (Variables|Default|GetPlane) (LocalVariables|GetNewOffset) false false)
  (Transformation|SetRelativeLocation (Variables|Default|GetBox) (LocalVariables|GetNewOffset) false false))

(fn UpdateTint
  (Rendering|Material|SetVectorParameterValue (Variables|Default|GetDynamicMaterialInstance) "TintColor" (Variables|Rendering|GetTintColor) :!class /Script/Engine.MaterialInstanceDynamic))