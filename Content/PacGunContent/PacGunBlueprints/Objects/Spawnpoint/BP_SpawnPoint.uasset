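; BP_SpawnPoint is a typed spawn marker that spawns a player start, weapon pickup, health item or page (Card type) at its location.
; Construction applies a dynamic beam material to a cylinder, colored by SpawnPointType.
; SpawnElement, not called within this Blueprint, dispatches on that type and stores the result in SpawnedActor.
; Weapons are random DT_Weapons rows excluding the pellet gun, and player starts are raised above the marker.
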(event EventBeginPlay)

(event Collision|EventActorBeginOverlap
  (params (OtherActor :type Actor%20Object%20Reference)))

(event EventTick
  (params (DeltaSeconds :type Float%20%28single-precision%29)))

(fn ConstructionScript
  (CallFunction|InitPlayerSpawn))

(fn SetBeamColor
  (Rendering|Material|SetVectorParameterValue (Variables|Default|GetDynamicMaterial) "Color" (CallFunction|GetBeamColor) :!class /Script/Engine.MaterialInstanceDynamic))

(fn InitPlayerSpawn
  (bind _returnvalue (Rendering|Material|CreateDynamicMaterialInstance (Variables|Default|GetBeamMaterial) "None" "None" :!class /Script/Engine.KismetMaterialLibrary))
  (bind _output_get (Variables|Default|SetDynamicMaterial _returnvalue))
  (Rendering|Material|SetMaterial (Variables|Default|GetCylinder) 0 _output_get)
  (CallFunction|SetBeamColor))

(fn GetBeamColor
  (switch Utilities|FlowControl|Switch|SwitchonE_SpawnPointType (Variables|Config|GetSpawnPointType)
    (:NewEnumerator4
      (return "(R=0.000000,G=0.000000,B=0.000000,A=1.000000)"))
    (:NewEnumerator0
      (return "(R=0.170517,G=1.000000,B=0.900265,A=1.000000)"))
    (:NewEnumerator1
      (return "(R=1.000000,G=0.211753,B=0.021443,A=1.000000)"))
    (:NewEnumerator2
      (return "(R=1.000000,G=0.000000,B=0.986205,A=1.000000)"))
    (:NewEnumerator3
      (return "(R=1.000000,G=0.000000,B=0.000000,A=1.000000)"))))

(fn SpawnWeapon
  (bind _outrownames (DataTable|GetDataTableRowNames "/Game/PacGunContent/PacGunBlueprints/Systems/WeaponSystem/DT_Weapons.DT_Weapons"))
  (bind _output_get (LocalVariables|SetWeaponsToSpawn _outrownames))
  (Utilities|Array|RemoveItem _output_get "pelletgun")
  (bind _returnvalue (Game|SpawnActorfromClass "/Game/PacGunContent/PacGunBlueprints/Systems/WeaponSystem/BP_WeaponPickup.BP_WeaponPickup_C" (Transformation|GetActorTransform) "Undefined" "MultiplyWithRoot" 0 (Utilities|Struct|MakeDataTableRowHandle "/Game/PacGunContent/PacGunBlueprints/Systems/WeaponSystem/DT_Weapons.DT_Weapons" (.OutItem (Utilities|Array|Random (LocalVariables|GetWeaponsToSpawn)))) 0))
  (Variables|Default|SetSpawnedActor _returnvalue)
  (return))

(fn SpawnElement
  (switch Utilities|FlowControl|Switch|SwitchonE_SpawnPointType (Variables|Config|GetSpawnPointType)
    (:NewEnumerator4
      (return))
    (:NewEnumerator0
      (CallFunction|SpawnPlayerStart)
      (return))
    (:NewEnumerator1
      (CallFunction|SpawnWeapon)
      (return))
    (:NewEnumerator2
      (CallFunction|SpawnItem))
    (:NewEnumerator3
      (CallFunction|SpawnCard))))

(fn SpawnItem
  (bind _returnvalue (Game|SpawnActorfromClass :Class "/Game/PacGunContent/PacGunBlueprints/Systems/WeaponSystem/BP_HealthyPax.BP_HealthyPax_C" :SpawnTransform (Transformation|GetActorTransform) :CollisionHandlingOverride "Undefined" :TransformScaleMethod "MultiplyWithRoot" :Instigator 0))
  (Variables|Default|SetSpawnedActor _returnvalue))

(fn SpawnCard
  (bind _returnvalue (Game|SpawnActorfromClass "/Game/PacGunContent/PacGunBlueprints/Objects/Cards/BP_Page.BP_Page_C" (Transformation|GetActorTransform) "AlwaysSpawn" "MultiplyWithRoot" 0 0))
  (Variables|Default|SetSpawnedActor _returnvalue))

(fn SpawnPlayerStart
  (bind _returnvalue (Transformation|GetActorTransform))
  (bind (_location _rotation) (Math|Transform|BreakTransform _returnvalue))
  (bind _returnvalue_2 (Game|SpawnActorfromClass "/Script/Engine.PlayerStart" (Math|Transform|MakeTransform (+ _location "0.000000,0.000000,100.000000") _rotation) "Undefined" "MultiplyWithRoot" 0 0))
  (Variables|Default|SetSpawnedActor _returnvalue_2))