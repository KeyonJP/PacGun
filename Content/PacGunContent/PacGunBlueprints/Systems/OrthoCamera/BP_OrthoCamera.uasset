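; Orthographic camera actor that keeps a fixed vertical world extent, set by top and bottom edge handles.
; The construction script derives screen height from the handles, recenters the actor between them on Y and repositions their visualizers.
; UpdateWidth multiplies that height by the viewport aspect ratio to set ortho width, running at construction, BeginPlay and every Tick.
; UpdateLocation is an empty stub.
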(event EventBeginPlay
  (bind _returnvalue (Transformation|GetActorLocation))
  (bind (_x _y _z) (Math|Vector|BreakVector _returnvalue))
  (CallFunction|UpdateWidth)
  ;[1 1 1] Set the actor location to be halfway between the two handles.
  (Transformation|SetActorLocation (Math|Vector|MakeVector _x (+ (Variables|Default|GetWorldTopEdge) (/ (Variables|Default|GetScreenHeight) 2.0)) _z) false false))

(event Collision|EventActorBeginOverlap
  (params (OtherActor :type Actor%20Object%20Reference)))

(event EventTick
  (params (DeltaSeconds :type Float%20%28single-precision%29))
  (CallFunction|UpdateWidth))

(fn ConstructionScript
  (bind _returnvalue (Transformation|GetActorLocation))
  (bind (_x _y _z) (Math|Vector|BreakVector _returnvalue))
  ;[1 1 1] Determine the world Y location of the top edge handle.
  (Variables|Default|SetWorldTopEdge (+ (.Y (Math|Vector|BreakVector (Transformation|GetActorLocation))) (.Y (Math|Vector|BreakVector (Variables|Config|GetTopEdge)))))
  ;[1 1 1] Determine the world Y location of the bottom edge handle.
  (Variables|Default|SetWorldBottomEdge (+ (.Y (Math|Vector|BreakVector (Transformation|GetActorLocation))) (.Y (Math|Vector|BreakVector (Variables|Config|GetBottomEdge)))))
  ;[1 1 1] Find the distance between the edges. This is the screen height.
  (Variables|Default|SetScreenHeight (- (Variables|Default|GetWorldBottomEdge) (Variables|Default|GetWorldTopEdge)))
  ;[1 1 1] Update the bottom handle value.
  (Variables|Config|SetBottomEdge (Math|Vector|MakeVector 0.0 (/ (Variables|Default|GetScreenHeight) 2.0) 0.0))
  ;[1 1 1] Update the top handle value.
  (Variables|Config|SetTopEdge (Math|Vector|MakeVector 0.0 (* (/ (Variables|Default|GetScreenHeight) 2.0) -1.0) 0.0))
  ;[1 1 1] Set the location of the handle visualizers.
  (Transformation|SetRelativeLocation (Variables|Default|GetTopPoint) (Variables|Config|GetTopEdge) false false)
  (Transformation|SetRelativeLocation (Variables|Default|GetBottomPoint) (Variables|Config|GetBottomEdge) false false)
  ;[1 1 1] Set the actor location to be halfway between the two handles.
  (Transformation|SetActorLocation (Math|Vector|MakeVector _x (+ (Variables|Default|GetWorldTopEdge) (/ (Variables|Default|GetScreenHeight) 2.0)) _z) false false)
  (CallFunction|UpdateWidth))

(fn UpdateWidth
  (bind _returnvalue (Viewport|GetViewportSize))
  (bind (_x _y) (Math|Vector2D|BreakVector2D _returnvalue))
  (Class|CameraComponent|SetOrthoWidth (Variables|Default|GetCamera) (* (Variables|Default|GetScreenHeight) (/ _x _y))))

(fn UpdateLocation)