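; BP_WeaponActorMaster is a base weapon actor that fires projectiles defined per weapon in DT_Weapons.
; StartPrimaryAttack checks the cooldown, looks up the WeaponIdentifier row, requests the projectile, starts the cooldown and returns success.
; LoadProjectile async-loads the projectile class, then spawns it at ProjectileSpawnpoint with the WeaponIdentifier.
; A timer lasting the row's ShotCooldown blocks further shots; PlayFlipbook is an empty stub.
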(event Custom|LoadProjectile
  (params (Projectile :type BP%20Projectile%20MASTER%20Soft%20Class%20Reference) (WeaponIdentifier :type Name))
  (bind _class (Utilities|AsyncLoadClassAsset Projectile)
    (:Completed
      (bind _asbp_projectile_master (Utilities|Casting|CastToBP_ProjectileMASTERClass _class))
      (Game|SpawnActorfromClass _asbp_projectile_master (Transformation|GetWorldTransform (Variables|Default|GetProjectileSpawnpoint)) "Undefined" 0 WeaponIdentifier 0))))

(event EventBeginPlay)

(event Collision|EventActorBeginOverlap
  (params (OtherActor :type Actor%20Object%20Reference)))

(event EventTick
  (params (DeltaSeconds :type Float%20%28single-precision%29)))

(fn ConstructionScript)

(fn StartPrimaryAttack
  (if (CallFunction|CanPrimaryAttack?)
    (bind _returnvalue (Utilities|GetDataTableRow "/Game/PacGunContent/PacGunBlueprints/Systems/WeaponSystem/DT_Weapons.DT_Weapons" (Variables|Default|GetWeaponIdentifier))
      (:then
        (CallFunction|LoadProjectile (Utilities|Struct|BreakS_DT_Weapons _returnvalue) (Variables|Default|GetWeaponIdentifier))
        (CallFunction|StartPrimaryCooldown)
        (return true))
      (:RowNotFound
        (return false)))
    (else
      (return false))))

(fn StartPrimaryCooldown
  (bind _returnvalue (Utilities|GetDataTableRow "/Game/PacGunContent/PacGunBlueprints/Systems/WeaponSystem/DT_Weapons.DT_Weapons" (Variables|Default|GetWeaponIdentifier))
    (:then
      (bind _returnvalue_2 (Utilities|Time|SetTimerbyFunctionName 0 "TimerFunc_PrimaryCooldown" (Utilities|Struct|BreakS_DT_Weapons _returnvalue)))
      (Variables|Default|SetPrimaryCooldownTimer _returnvalue_2)
      (return))
    (:RowNotFound
      (return))))

(fn TimerFuncPrimaryCooldown
  (Utilities|Time|ClearandInvalidateTimerbyHandle (Variables|Default|GetPrimaryCooldownTimer))
  (return))

(fn CanPrimaryAttack?
  (return (not (Utilities|Time|IsTimerActivebyHandle (Variables|Default|GetPrimaryCooldownTimer)))))

(fn PlayFlipbook)