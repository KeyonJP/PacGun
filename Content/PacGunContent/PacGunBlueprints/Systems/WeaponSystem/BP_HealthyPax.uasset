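; BP_HealthyPax is a health pickup that restores a small fixed amount of HP to the ghost hunter character.
; Each Tick it billboards its flipbook sprite toward the player camera using look-at pitch and offset yaw.
; When the character overlaps its sphere, it adds HP clamped to the maximum, updates the HUD health bar, plays a pickup sound and destroys itself.
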(event OnComponentBeginOverlap(Sphere)
  (params (OverlappedComponent :type Primitive%20Component%20Object%20Reference) (OtherActor :type Actor%20Object%20Reference) (OtherComp :type Primitive%20Component%20Object%20Reference) (OtherBodyIndex :type Integer) (bFromSweep :type Boolean) (SweepResult :type Hit%20Result%20Structure%20%28by%20ref%29))
  (bind _asbp_ghost_hunter_character (Utilities|Casting|CastToBP_GhostHunterCharacter OtherActor))
  (bind _output_get (Variables|/Game/PacGunContent/PacGunBlueprints/PacGunFramework/GhostHunt/BP_GhostHunterCharacter.BP_GhostHunterCharacter_C|SetHP_Current _asbp_ghost_hunter_character (Math|Float|Clamp(Float) (+ (Variables|/Game/PacGunContent/PacGunBlueprints/PacGunFramework/GhostHunt/BP_GhostHunterCharacter.BP_GhostHunterCharacter_C|GetHP_Current _asbp_ghost_hunter_character) 5.0) 0.0 (Variables|/Game/PacGunContent/PacGunBlueprints/PacGunFramework/GhostHunt/BP_GhostHunterCharacter.BP_GhostHunterCharacter_C|GetHP_Maximum _asbp_ghost_hunter_character))))
  (Default|ChangeHealthbar (Variables|/Game/PacGunContent/PacGunBlueprints/PacGunFramework/GhostHunt/BP_GhostHunterCharacter.BP_GhostHunterCharacter_C|GetMainHUD _asbp_ghost_hunter_character) true _output_get (Variables|/Game/PacGunContent/PacGunBlueprints/PacGunFramework/GhostHunt/BP_GhostHunterCharacter.BP_GhostHunterCharacter_C|GetHP_Maximum _asbp_ghost_hunter_character))
  (Audio|PlaySound2D "/Game/Retro_8Bit_Sounds/Collectables/Wavs/retro_collect_pickup_coin_14.retro_collect_pickup_coin_14" 1.0 1.0 0.0 0 0)
  (Actor|DestroyActor))

(event EventBeginPlay
  (|CallParentFunction) ; This node is disabled and will not be called.\nDrag off pins to build functionality.
)

(event Collision|EventActorBeginOverlap
  (params (OtherActor :type Actor%20Object%20Reference))
  (|CallParentFunction OtherActor) ; This node is disabled and will not be called.\nDrag off pins to build functionality.
)

(event EventTick
  (params (DeltaSeconds :type Float%20%28single-precision%29))
  (bind _returnvalue (Game|GetPlayerCameraManager 0))
  (bind _flipbook_pickup_healthypack (Variables|Default|GetFlipbook_PickUp_HealthyPack))
  (bind _returnvalue_2 (Camera|GetCameraLocation _returnvalue))
  (bind _returnvalue_3 (Transformation|GetWorldLocation _flipbook_pickup_healthypack))
  (bind _returnvalue_4 (Math|Rotator|FindLookatRotation _returnvalue_3 _returnvalue_2))
  (bind (_roll _pitch _yaw) (Math|Rotator|BreakRotator _returnvalue_4))
  (Transformation|SetRelativeRotation (Variables|Default|GetFlipbook_PickUp_HealthyPack) (Math|Rotator|MakeRotator 0.0 _pitch (+ _yaw 9e+01)) false false))

(fn ConstructionScript
  (|CallParentFunction))