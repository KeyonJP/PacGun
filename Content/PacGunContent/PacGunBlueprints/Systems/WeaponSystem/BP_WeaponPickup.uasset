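; BP_WeaponPickup is a spinning sprite pickup that equips a weapon on a BP_GhostHunterCharacter that overlaps its sphere.
; The construction script looks up the Weapon row in DT_Weapons to set the sprite, and overlap passes that row name to EquipWeapon.
; Tick yaws the sprite by RotationSpeed divided by DeltaSeconds, so spin speed depends on frame rate.
; The pickup does not destroy or disable itself after use.
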(event OnComponentBeginOverlap(Sphere)
  (params (OverlappedComponent :type Primitive%20Component%20Object%20Reference) (OtherActor :type Actor%20Object%20Reference) (OtherComp :type Primitive%20Component%20Object%20Reference) (OtherBodyIndex :type Integer) (bFromSweep :type Boolean) (SweepResult :type Hit%20Result%20Structure%20%28by%20ref%29))
  (bind _asbp_ghost_hunter_character (Utilities|Casting|CastToBP_GhostHunterCharacter OtherActor))
  (Default|EquipWeapon _asbp_ghost_hunter_character (.RowName (Utilities|Struct|BreakDataTableRowHandle (Variables|Pickup|GetWeapon)))))

(event EventBeginPlay)

(event Collision|EventActorBeginOverlap
  (params (OtherActor :type Actor%20Object%20Reference)))

(event EventTick
  (params (DeltaSeconds :type Float%20%28single-precision%29))
  (bind _papersprite (Variables|Default|GetPaperSprite))
  (bind _returnvalue (Transformation|GetWorldRotation _papersprite))
  (Transformation|SetWorldRotation (Variables|Default|GetPaperSprite) (Math|Rotator|MakeRotator (.roll _returnvalue) (.pitch _returnvalue) (+ (.yaw _returnvalue) (/ (Variables|Pickup|GetRotationSpeed) DeltaSeconds))) false false))

(fn ConstructionScript
  (bind _returnvalue (Utilities|GetDataTableRow "/Game/PacGunContent/PacGunBlueprints/Systems/WeaponSystem/DT_Weapons.DT_Weapons" (.RowName (Utilities|Struct|BreakDataTableRowHandle (Variables|Pickup|GetWeapon))))
    (:then
      (Rendering|Components|Sprite|SetSprite (Variables|Default|GetPaperSprite) (.WeaponSprite (Utilities|Struct|BreakS_DT_Weapons _returnvalue))))))