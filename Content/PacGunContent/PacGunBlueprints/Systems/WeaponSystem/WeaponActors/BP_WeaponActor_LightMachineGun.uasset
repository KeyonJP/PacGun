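; BP_WeaponActor_LightMachineGun is a child weapon actor for the light machine gun that adds a visual recoil kick when it fires.
; StartPrimaryAttack calls the parent attack and triggers GunRecoilVisual only if that attack succeeds, passing the result back to the caller.
; GunRecoilVisual plays a timeline from the start to drive the GunOffset component's relative location and rotation, then zeroes both when finished.
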(event Custom|GunRecoilVisual
  (bind _gunoffset (Variables|Default|GetGunOffset))
  (bind _gunoffset_2 (Variables|Default|GetGunOffset))
  (bind (_direction _rotationoffset _locationoffset) (Timeline|Timeline PlayFromStart)
    (:Update
      (Transformation|SetRelativeLocation _gunoffset_2 _locationoffset false false)
      (Transformation|SetRelativeRotation _gunoffset_2 (Math|Rotator|MakeRotator (.X (Math|Vector|BreakVector _rotationoffset)) (.Y (Math|Vector|BreakVector _rotationoffset)) (.Z (Math|Vector|BreakVector _rotationoffset))) false false))
    (:Finished
      (Transformation|SetRelativeLocation _gunoffset "0, 0, 0" false false)
      (Transformation|SetRelativeRotation _gunoffset "0, 0, 0" false false))))

(event EventBeginPlay)

(event Collision|EventActorBeginOverlap
  (params (OtherActor :type Actor%20Object%20Reference)))

(event EventTick
  (params (DeltaSeconds :type Float%20%28single-precision%29)))

(fn ConstructionScript
  (|CallParentFunction))

(fn StartPrimaryAttack
  (bind _success_ (|CallParentFunction))
  (if _success_
    (CallFunction|GunRecoilVisual)
    (return true)
    (else
      (return _success_))))