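; Shotgun weapon actor, a child Blueprint that adds a spin animation to the weapon's sprite when it attacks.
; It overrides StartPrimaryAttack to call the parent logic and, only if that succeeds, fire StartSpin before returning the result.
; StartSpin replays the Spin timeline from the start, driving the PaperSprite's relative pitch on each update.
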(event Custom|StartSpin
  (Utilities|FlowControl|Sequence
    (:then_0
      (bind _spin (Timeline|Spin PlayFromStart)
        (:Update
          (Transformation|SetRelativeRotation (Variables|Default|GetPaperSprite) (Math|Rotator|MakeRotator 0.0 _spin 0.0) false false))))))

(event EventBeginPlay)

(event Collision|EventActorBeginOverlap
  (params (OtherActor :type Actor%20Object%20Reference)))

(event EventTick
  (params (DeltaSeconds :type Float%20%28single-precision%29)))

(fn ConstructionScript
  (|CallParentFunction))

(fn StartPrimaryAttack
  (bind _success_ (|CallParentFunction))
  (if _success_
    (CallFunction|StartSpin)
    (return true)
    (else
      (return _success_))))