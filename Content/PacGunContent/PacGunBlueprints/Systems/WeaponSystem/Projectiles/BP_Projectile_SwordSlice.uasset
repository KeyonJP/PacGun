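; Sword slice attack built as a short-lived projectile actor that deals instant area damage to Ghosts in front of it.
; On BeginPlay it sizes and offsets a box hitbox forward, then plays a camera shake and a random slash sound.
; It reads damage from DT_Weapons by weapon identifier, damages every overlapping Ghost with a random impact sound, then destroys itself without travelling.
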(event EventBeginPlay
  (bind _returnvalue (Transformation|GetActorLocation))
  (bind _returnvalue_2 (Transformation|GetActorLocation))
  (Variables|Default|SetWidth 3e+02)
  (Variables|Default|SetDistance 1.5e+02)
  (CallFunction|UpdateHitbox)
  (CameraShakes|StartCameraShake (Game|GetPlayerCameraManager 0) "/Game/PacGunContent/PacGunBlueprints/PacGunFramework/GhostHunt/ShotCameraShake.ShotCameraShake_C" 1.0 "CameraLocal" "0, 0, 0")
  (switch int (Math|Random|RandomIntegerinRange 0 2)
    (:0
      (Audio|PlaySoundatLocation "/Game/Retro_8Bit_Sounds/Weapons/Wavs/retro_laser_gun_shoot_52.retro_laser_gun_shoot_52" _returnvalue "0, 0, 0" 1.0 1.0 0.0 0 0 0 0))
    (:1
      (Audio|PlaySoundatLocation "/Game/Retro_8Bit_Sounds/Weapons/Wavs/retro_laser_gun_shoot_53.retro_laser_gun_shoot_53" _returnvalue "0, 0, 0" 1.0 1.0 0.0 0 0 0 0))
    (:2
      (Audio|PlaySoundatLocation "/Game/Retro_8Bit_Sounds/Weapons/Wavs/retro_laser_gun_shoot_54.retro_laser_gun_shoot_54" _returnvalue "0, 0, 0" 1.0 1.0 0.0 0 0 0 0)))
  (bind _returnvalue_3 (Utilities|GetDataTableRow "/Game/PacGunContent/PacGunBlueprints/Systems/WeaponSystem/DT_Weapons.DT_Weapons" (Variables|Default|GetWeaponIdentifier))
    (:then
      (for _array_element (Collision|GetOverlappingActors (Variables|Default|GetBox) 0 :!class /Script/Engine.PrimitiveComponent)
        (bind _asghost (Utilities|Casting|CastToGhost _array_element))
        (Game|Damage|ApplyDamage _asghost (.ProjectileDamage (Utilities|Struct|BreakS_DT_Weapons _returnvalue_3)) (Game|GetPlayerController 0) self)
        (switch int (Math|Random|RandomIntegerinRange 0 2)
          (:0
            (Audio|PlaySoundatLocation "/Game/Retro_8Bit_Sounds/Impacts/Wavs/retro_impact_colorful_07.retro_impact_colorful_07" _returnvalue_2 "0, 0, 0" 1.0 1.0 0.0 0 0 0 0))
          (:1
            (Audio|PlaySoundatLocation "/Game/Retro_8Bit_Sounds/Impacts/Wavs/retro_impact_colorful_08.retro_impact_colorful_08" _returnvalue_2 "0, 0, 0" 1.0 1.0 0.0 0 0 0 0))
          (:2
            (Audio|PlaySoundatLocation "/Game/Retro_8Bit_Sounds/Impacts/Wavs/retro_impact_colorful_09.retro_impact_colorful_09" _returnvalue_2 "0, 0, 0" 1.0 1.0 0.0 0 0 0 0))))
      (Actor|DestroyActor))))

(fn ConstructionScript)

(fn UpdateHitbox
  (bind _width (Variables|Default|GetWidth))
  (Components|Box|SetBoxExtent (Variables|Default|GetBox) (Math|Vector|MakeVector (Variables|Default|GetDistance) _width _width) true)
  (Transformation|SetRelativeLocation (Variables|Default|GetBox) (Math|Vector|MakeVector (/ (Variables|Default|GetDistance) 2.0) 0.0 0.0) false false))