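; Pellet shot projectile that damages what it hits and lives at most one second.
; On spawn it shakes the camera, plays a random shot sound and immediately hits any Ghost already overlapping its sphere.
; Later overlaps ignore the player; world-object hits search a wider sphere for a Ghost before giving up, making aim forgiving.
; Hits play a random impact sound, apply damage from the weapon's DT_Weapons row and destroy the pellet.
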(event OnComponentBeginOverlap(CollisionSphere)
  (params (OverlappedComponent :type Primitive%20Component%20Object%20Reference) (OtherActor :type Actor%20Object%20Reference) (OtherComp :type Primitive%20Component%20Object%20Reference) (OtherBodyIndex :type Integer) (bFromSweep :type Boolean) (SweepResult :type Hit%20Result%20Structure%20%28by%20ref%29))
  (bind _returnvalue (Transformation|GetActorLocation))
  (Variables|Default|SetHitComponet OtherComp)
  (Variables|Default|SetHitActor OtherActor)
  (Utilities|Casting|CastToBP_GhostHunterCharacter OtherActor
    (:CastFailed
      (if (or (Utilities|Enum|Equal(Enum) (Collision|GetCollisionObjectType (Variables|Default|GetHitComponet)) "ECC_WorldStatic") (Utilities|Enum|Equal(Enum) (Collision|GetCollisionObjectType (Variables|Default|GetHitComponet)) "ECC_WorldDynamic"))
        (bind _outactors (Collision|SphereOverlapActors (Transformation|GetWorldLocation (Variables|Default|GetCollisionSphere)) (* (Variables|/Script/Engine.SphereComponent|GetSphereRadius (Variables|Default|GetCollisionSphere)) 2.3) (Utilities|Array|MakeArray "ObjectTypeQuery3") "/Game/PacGunContent/PacGunBlueprints/Objects/Enemy/Ghost/Ghost.Ghost_C"))
        (if (> (Utilities|Array|Length _outactors) 0)
          (Variables|Default|SetHitActor (Utilities|Array|Get(acopy) _outactors))
          (switch int (Math|Random|RandomIntegerinRange 0 2) :!label _label
            (:0
              (Audio|PlaySoundatLocation "/Game/Retro_8Bit_Sounds/Impacts/Wavs/retro_impact_colorful_07.retro_impact_colorful_07" _returnvalue "0, 0, 0" 1.0 1.0 0.0 0 0 0 0))
            (:1
              (Audio|PlaySoundatLocation "/Game/Retro_8Bit_Sounds/Impacts/Wavs/retro_impact_colorful_08.retro_impact_colorful_08" _returnvalue "0, 0, 0" 1.0 1.0 0.0 0 0 0 0))
            (:2
              (Audio|PlaySoundatLocation "/Game/Retro_8Bit_Sounds/Impacts/Wavs/retro_impact_colorful_09.retro_impact_colorful_09" _returnvalue "0, 0, 0" 1.0 1.0 0.0 0 0 0 0)))
          (bind _returnvalue_2 (Utilities|GetDataTableRow "/Game/PacGunContent/PacGunBlueprints/Systems/WeaponSystem/DT_Weapons.DT_Weapons" (Variables|Default|GetWeaponIdentifier))
            (:then
              (Game|Damage|ApplyDamage (Variables|Default|GetHitActor) (.ProjectileDamage (Utilities|Struct|BreakS_DT_Weapons _returnvalue_2)) (Game|GetPlayerController 0) self)
              (Actor|DestroyActor)))
          (else
            (Actor|DestroyActor)))
        (else
          (goto _label))))))

(event EventBeginPlay
  (bind _returnvalue (Transformation|GetActorLocation))
  (bind _returnvalue_2 (Transformation|GetActorLocation))
  (bind _collisionsphere (Variables|Default|GetCollisionSphere))
  (bind _overlappingactors (Collision|GetOverlappingActors _collisionsphere "/Game/PacGunContent/PacGunBlueprints/Objects/Enemy/Ghost/Ghost.Ghost_C" :!class /Script/Engine.PrimitiveComponent))
  (CameraShakes|StartCameraShake (Game|GetPlayerCameraManager 0) "/Game/PacGunContent/PacGunBlueprints/PacGunFramework/GhostHunt/ShotCameraShake.ShotCameraShake_C" 1.0 "CameraLocal" "0, 0, 0")
  (switch int (Math|Random|RandomIntegerinRange 0 2)
    (:0
      (Audio|PlaySoundatLocation "/Game/Retro_8Bit_Sounds/Weapons/Wavs/retro_laser_gun_shoot_52.retro_laser_gun_shoot_52" _returnvalue "0, 0, 0" 1.0 1.0 0.0 0 0 0 0))
    (:1
      (Audio|PlaySoundatLocation "/Game/Retro_8Bit_Sounds/Weapons/Wavs/retro_laser_gun_shoot_53.retro_laser_gun_shoot_53" _returnvalue "0, 0, 0" 1.0 1.0 0.0 0 0 0 0))
    (:2
      (Audio|PlaySoundatLocation "/Game/Retro_8Bit_Sounds/Weapons/Wavs/retro_laser_gun_shoot_54.retro_laser_gun_shoot_54" _returnvalue "0, 0, 0" 1.0 1.0 0.0 0 0 0 0)))
  (Utilities|FlowControl|Sequence
    (:then_0
      (Utilities|FlowControl|Delay 1.0)
      (Actor|DestroyActor))
    (:then_1
      (if (> (Utilities|Array|Length _overlappingactors) 0)
        (Variables|Default|SetHitActor (Utilities|Array|Get(acopy) _overlappingactors))
        (switch int (Math|Random|RandomIntegerinRange 0 2)
          (:0
            (Audio|PlaySoundatLocation "/Game/Retro_8Bit_Sounds/Impacts/Wavs/retro_impact_colorful_07.retro_impact_colorful_07" _returnvalue_2 "0, 0, 0" 1.0 1.0 0.0 0 0 0 0))
          (:1
            (Audio|PlaySoundatLocation "/Game/Retro_8Bit_Sounds/Impacts/Wavs/retro_impact_colorful_08.retro_impact_colorful_08" _returnvalue_2 "0, 0, 0" 1.0 1.0 0.0 0 0 0 0))
          (:2
            (Audio|PlaySoundatLocation "/Game/Retro_8Bit_Sounds/Impacts/Wavs/retro_impact_colorful_09.retro_impact_colorful_09" _returnvalue_2 "0, 0, 0" 1.0 1.0 0.0 0 0 0 0)))
        (bind _returnvalue_3 (Utilities|GetDataTableRow "/Game/PacGunContent/PacGunBlueprints/Systems/WeaponSystem/DT_Weapons.DT_Weapons" (Variables|Default|GetWeaponIdentifier))
          (:then
            (Game|Damage|ApplyDamage (Variables|Default|GetHitActor) (.ProjectileDamage (Utilities|Struct|BreakS_DT_Weapons _returnvalue_3)) (Game|GetPlayerController 0) self)
            (Actor|DestroyActor)))))))

(fn ConstructionScript)