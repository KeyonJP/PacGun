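; Rocket projectile for the weapon system that explodes on overlap and damages nearby ghosts.
; On spawn it shakes the camera, plays a random launch sound and destroys itself after one second.
; Overlapping anything but the ghost hunter character applies DT_Weapons damage to ghosts inside ExplosionCollision.
; It then stops, plays a random blast sound and scales an explosion sphere by timeline before destroying itself.
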(event OnComponentBeginOverlap(CollisionSphere)
  (params (OverlappedComponent :type Primitive%20Component%20Object%20Reference) (OtherActor :type Actor%20Object%20Reference) (OtherComp :type Primitive%20Component%20Object%20Reference) (OtherBodyIndex :type Integer) (bFromSweep :type Boolean) (SweepResult :type Hit%20Result%20Structure%20%28by%20ref%29))
  (bind _returnvalue (Transformation|GetActorLocation))
  (Variables|Default|SetHitComponet OtherComp)
  (bind _output_get (Variables|Default|SetHitActor OtherActor))
  (Utilities|Casting|CastToBP_GhostHunterCharacter _output_get
    (:CastFailed
      (Rendering|SetVisibility (Variables|Default|GetRocketRoot) false true)
      (bind _returnvalue_2 (Utilities|GetDataTableRow "/Game/PacGunContent/PacGunBlueprints/Systems/WeaponSystem/DT_Weapons.DT_Weapons" (Variables|Default|GetWeaponIdentifier))
        (:then
          (bind _output_get_2 (Variables|Default|SetOverlapping%20Actors (Collision|GetOverlappingActors (Variables|Default|GetExplosionCollision) "/Game/PacGunContent/PacGunBlueprints/Objects/Enemy/Ghost/Ghost.Ghost_C" :!class /Script/Engine.PrimitiveComponent)))
          (for _array_element _output_get_2
            (Game|Damage|ApplyDamage _array_element (.ProjectileDamage (Utilities|Struct|BreakS_DT_Weapons _returnvalue_2)) (Game|GetPlayerController 0) self))
          (switch int (Math|Random|RandomIntegerinRange 0 1)
            (:0
              (Audio|PlaySoundatLocation "/Game/Retro_8Bit_Sounds/Explosion/Cues/retro_explosion_bass_03_Cue.retro_explosion_bass_03_Cue" _returnvalue "0, 0, 0" 1.0 1.0 0.0 0 0 0 0))
            (:1
              (Audio|PlaySoundatLocation "/Game/Retro_8Bit_Sounds/Explosion/Cues/retro_explosion_bass_09_Cue.retro_explosion_bass_09_Cue" _returnvalue "0, 0, 0" 1.0 1.0 0.0 0 0 0 0)))
          (Rendering|SetVisibility (Variables|Default|GetRocketRoot) false false)
          (Collision|SetCollisionEnabled (Variables|Default|GetCollisionSphere) "NoCollision")
          (Components|Movement|StopMovementImmediately (Variables|Default|GetProjectileMovement))
          (Rendering|SetVisibility (Variables|Default|GetExplosionSphere_0) true false)
          (bind _spherescale (Timeline|Explosion PlayFromStart)
            (:Update
              (Transformation|SetRelativeScale3D (Variables|Default|GetExplosionSphere_0) (Math|Vector|MakeVector _spherescale _spherescale _spherescale)))
            (:Finished
              (Actor|DestroyActor))))))))

(event EventBeginPlay
  (bind _returnvalue (Transformation|GetActorLocation))
  (CameraShakes|StartCameraShake (Game|GetPlayerCameraManager 0) "/Game/PacGunContent/PacGunBlueprints/PacGunFramework/GhostHunt/ShotCameraShake.ShotCameraShake_C" 1.0 "CameraLocal" "0, 0, 0")
  (switch int (Math|Random|RandomIntegerinRange 0 1)
    (:0
      (Audio|PlaySoundatLocation "/Game/Retro_8Bit_Sounds/Explosion/Cues/retro_explosion_deep_01_Cue.retro_explosion_deep_01_Cue" _returnvalue "0, 0, 0" 2.0 1.0 0.0 0 0 0 0))
    (:1
      (Audio|PlaySoundatLocation "/Game/Retro_8Bit_Sounds/Explosion/Cues/retro_explosion_deep_09_Cue.retro_explosion_deep_09_Cue" _returnvalue "0, 0, 0" 2.0 1.0 0.0 0 0 0 0)))
  (Utilities|FlowControl|Delay 1.0)
  (Actor|DestroyActor))

(fn ConstructionScript)