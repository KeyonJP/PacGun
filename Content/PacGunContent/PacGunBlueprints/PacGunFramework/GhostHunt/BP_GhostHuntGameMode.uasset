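; Game mode for Ghost Hunt that populates the level from spawn points and starts players at a random PlayerStart.
; BeginPlay and FindPlayerStart both trigger a one-time SpawnOthers, so whichever runs first does the spawning.
; It shuffles all BP_SpawnPoint actors and tells each to spawn while its type is under a per-type cap, with a default fallback.
; Used points are removed from the valid list during iteration, shifting later indices.
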(event EventBeginPlay
  (CallFunction|SpawnOthers))

(event EventTick
  (params (DeltaSeconds :type Float%20%28single-precision%29)))

(fn ConstructionScript)

(fn FindPlayerStart
  (params (Player :type Controller%20Object%20Reference) (IncomingName :type String))
  (CallFunction|SpawnOthers)
  (bind _outactors (Actor|GetAllActorsOfClass "/Script/Engine.PlayerStart"))
  (return (.OutItem (Utilities|Array|Random _outactors))))

(fn SpawnOthers
  (if (not (Variables|Default|GetSpawned))
    (Variables|Default|SetSpawned true)
    (CallFunction|FindSpawnpoints)
    (Variables|Default|SetSpawnCountCurrent (Utilities|Map|MakeMap))
    (for (_array_element _array_index) (Variables|Default|GetValidSpawnpoints)
      ;[1 1 1] Get spawnpoints type.
      (bind _output_get (LocalVariables|SetSpawnpointType (Variables|/Game/PacGunContent/PacGunBlueprints/Objects/Spawnpoint/BP_SpawnPoint.BP_SpawnPoint_C|GetSpawnPointType _array_element)))
      ;[1 1 1] Detemine the maximum spawn count for the type of the current spawnpoint
      (LocalVariables|SetCurrentSpawnMax (Math|Integer|SelectInt (.Value (Utilities|Map|Find (Variables|Default|GetSpawnCountMax) _output_get)) (Variables|Default|GetDefaultSpawnCountMax) (.ReturnValue (Utilities|Map|Find (Variables|Default|GetSpawnCountMax) _output_get))))
      ;[1 1 1] Determine the current amount of the given type that are spawned.
      (LocalVariables|SetCurrentSpawnNumber (Math|Integer|SelectInt (.Value (Utilities|Map|Find (Variables|Default|GetSpawnCountCurrent) (LocalVariables|GetSpawnpointType))) 0 (.ReturnValue (Utilities|Map|Find (Variables|Default|GetSpawnCountCurrent) (LocalVariables|GetSpawnpointType)))))
      ;[1 1 1] Determine if we can spawn more of the given type.
      (if (< (LocalVariables|GetCurrentSpawnNumber) (LocalVariables|GetCurrentSpawnMax))
        (Default|SpawnElement _array_element)
        ;[1 1 1] Remove this spawnpoint from the list of valid spawnpoints
        (Utilities|Array|RemoveIndex (Variables|Default|GetValidSpawnpoints) _array_index)
        ;[1 1 1] Increment spawn count
        (Utilities|Map|Add (Variables|Default|GetSpawnCountCurrent) (LocalVariables|GetSpawnpointType) (+ (LocalVariables|GetCurrentSpawnNumber) 1))))
    (return)))

(fn FindSpawnpoints
  (bind _outactors (Actor|GetAllActorsOfClass "/Game/PacGunContent/PacGunBlueprints/Objects/Spawnpoint/BP_SpawnPoint.BP_SpawnPoint_C"))
  (bind _output_get (Variables|Default|SetValidSpawnpoints _outactors))
  (Utilities|Array|Shuffle _output_get))