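; Backdrop mountain plane actor that builds a tinted, optionally flipped mountain sprite when constructed.
; A dynamic material receives the texture, two colors and color distribution.
; It uses a dedicated mesh if set, otherwise a displacement-material default plane sized from the texture.
; With a UseCenter actor, it places itself around that center by angle, distance and height, yaws toward it, and adds the center's offsets, including scale.
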(event EventBeginPlay)

(event Collision|EventActorBeginOverlap
  (params (OtherActor :type Actor%20Object%20Reference)))

(event EventTick
  (params (DeltaSeconds :type Float%20%28single-precision%29)))

(fn ConstructionScript
  (CallFunction|MakeMaterial)
  (CallFunction|UpdateMaterial)
  (CallFunction|UpdatePlane)
  (CallFunction|UpdatePosition))

(fn UpdateMaterial
  (Utilities|IsValid (Variables|Default|GetDynamicMaterialInstance)
    (:Is%20Valid
      (Rendering|Material|SetTextureParameterValue (Variables|Default|GetDynamicMaterialInstance) "SpriteTexture" (Variables|Config|GetTexture))
      (Class|MaterialInstanceDynamic|SetVectorParameterValuebyInfo (Variables|Default|GetDynamicMaterialInstance) (Utilities|Struct|MakeMaterialParameterInfo "Color1" "GlobalParameter" -1) (Variables|Config|GetColor1))
      (Class|MaterialInstanceDynamic|SetVectorParameterValuebyInfo (Variables|Default|GetDynamicMaterialInstance) (Utilities|Struct|MakeMaterialParameterInfo "Color2" "GlobalParameter" -1) (Variables|Config|GetColor2))
      (Rendering|Material|SetScalarParameterValue (Variables|Default|GetDynamicMaterialInstance) "Power" (Variables|Config|GetColorDist) :!class /Script/Engine.MaterialInstanceDynamic))))

(fn UpdatePlane
  (Utilities|IsValid (Variables|Config|GetMesh)
    (:Is%20Valid
      (Components|StaticMesh|SetStaticMesh (Variables|Default|GetStaticMesh) (Variables|Config|GetMesh))
      (Transformation|SetRelativeScale3D (Variables|Default|GetStaticMesh) (Math|Vector|MakeVector (Variables|Config|GetDepth) (Math|Float|SelectFloat -2.0 2.0 (Variables|Config|GetIsFlipped)) 2.0)))
    (:Is%20Not%20Valid
      (Components|StaticMesh|SetStaticMesh (Variables|Default|GetStaticMesh) "/Game/PolyContent/Assets/Props/Nature/Mountians/SM_MountianPlane_SM_MountianPlaneTextures.SM_MountianPlane_SM_MountianPlaneTextures")
      (LocalVariables|SetSizeX (Class|Texture2D|BlueprintGetSizeX (Variables|Config|GetTexture)))
      (LocalVariables|SetSizeY (Class|Texture2D|BlueprintGetSizeY (Variables|Config|GetTexture)))
      (Transformation|SetRelativeScale3D (Variables|Default|GetStaticMesh) (Math|Vector|MakeVector (Variables|Config|GetDepth) (* (/ (Math|Conversions|ToFloat(Integer) (LocalVariables|GetSizeY)) 37.0) (* (/ (LocalVariables|GetSizeX) (LocalVariables|GetSizeY)) (Math|Float|SelectFloat -1.0 1.0 (Variables|Config|GetIsFlipped)))) (/ (Math|Conversions|ToFloat(Integer) (LocalVariables|GetSizeY)) 37.0)))))
  (Transformation|SetRelativeLocation (Variables|Default|GetStaticMesh) (Math|Vector|MakeVector 0.0 (Variables|Circle|GetShift) 0.0) false false))

(fn MakeMaterial
  (bind _returnvalue (Rendering|Material|CreateDynamicMaterialInstance (select (Utilities|IsValid (Variables|Config|GetMesh)) "/Game/PolyContent/Assets/Props/Nature/Mountians/M_MountianPlane_DedicatedMesh.M_MountianPlane_DedicatedMesh" "/Game/PolyContent/Assets/Props/Nature/Mountians/M_MountianPlane_Displacement.M_MountianPlane_Displacement") "None" "None" :!class /Script/Engine.KismetMaterialLibrary))
  (Variables|Default|SetDynamicMaterialInstance _returnvalue)
  (Rendering|Material|SetMaterial (Variables|Default|GetStaticMesh) 0 (Variables|Default|GetDynamicMaterialInstance))
  (return))

(fn UpdatePosition
  (bind _scale (Variables|Circle|GetScale))
  (bind _usecenter (Variables|Circle|GetUseCenter))
  (bind _scale_2 (Variables|/Game/PolyContent/Assets/BackdropSprites/BP_BackdropCircle.BP_BackdropCircle_C|GetScale _usecenter))
  (bind _returnvalue (+ _scale _scale_2))
  (Utilities|IsValid (Variables|Circle|GetUseCenter)
    (:Is%20Valid
      (bind _output_get (LocalVariables|SetLocation (+ (+ (* (Math|Vector|RotateVector (Transformation|GetActorForwardVector (Variables|Circle|GetUseCenter)) (Math|Rotator|MakeRotator 0.0 0.0 (Variables|Circle|GetAngle))) (+ (Variables|Circle|GetDistance) (Variables|/Game/PolyContent/Assets/BackdropSprites/BP_BackdropCircle.BP_BackdropCircle_C|GetDistance (Variables|Circle|GetUseCenter)))) (Transformation|GetActorLocation (Variables|Circle|GetUseCenter))) (Math|Vector|MakeVector 0.0 0.0 (+ (Variables|Circle|GetHeight) (Variables|/Game/PolyContent/Assets/BackdropSprites/BP_BackdropCircle.BP_BackdropCircle_C|GetHeight (Variables|Circle|GetUseCenter)))))))
      (Transformation|SetActorLocation _output_get false false)
      (Transformation|SetActorRotation (Math|Rotator|MakeRotator (.Roll (Math|Rotator|BreakRotator (Math|Rotator|FindLookatRotation (LocalVariables|GetLocation) (Transformation|GetActorLocation (Variables|Circle|GetUseCenter))))) (Variables|Circle|GetTilt) (.Yaw (Math|Rotator|BreakRotator (Math|Rotator|FindLookatRotation (LocalVariables|GetLocation) (Transformation|GetActorLocation (Variables|Circle|GetUseCenter)))))))
      (Transformation|SetActorScale3D (Math|Vector|MakeVector _returnvalue _returnvalue _returnvalue)))))

(fn UpdateAll
  (CallFunction|UpdatePosition)
  (CallFunction|UpdatePlane))